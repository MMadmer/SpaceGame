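; BP_SGPlayerState is the space game's player state, keeping a count of cleared "Mama" for the player.
; AddClearedMama adds positive amounts to the count and fires the OnMamaChanged dispatcher.
; The state binds to its own dispatcher on BeginPlay and forwards the new total to the player controller's HUD through the BPI_PlayerHUD interface, after validity checks.
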(event Custom|OnMamaChanged_Event
  (bind _returnvalue (Game|GetPlayerController))
  (bind _returnvalue_2 (HUD|GetHUD _returnvalue))
  (Utilities|IsValid _returnvalue
    (:Is%20Valid
      (Utilities|IsValid _returnvalue_2
        (:Is%20Valid
          (Utilities|ImplementsInterface _returnvalue_2 "/Game/SpaceGame/GameLogic/Blueprints/Interfaces/BPI_PlayerHUD.BPI_PlayerHUD_C"
            (:True
              (Class|BPIPlayerHUD|OnMamaChanged(Message) _returnvalue_2 (Variables|Default|GetClearedMama)))))))))

(event EventBeginPlay
  (EventDispatchers|AssignOnMamaChanged (delegate Custom|OnMamaChanged_Event)))

(fn ConstructionScript)

(fn AddClearedMama
  (params (Count :type Integer))
  (if (> Count 0)
    (Variables|Default|SetClearedMama (+ (Variables|Default|GetClearedMama) Count))
    (Default|CallOnMamaChanged)))