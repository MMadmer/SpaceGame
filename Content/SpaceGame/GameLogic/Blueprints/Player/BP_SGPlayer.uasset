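; BP_SGPlayer is the player character, handling movement, interaction, melee attack, blocking and cleaning animation.
; Input overrides and movement events drive the anim instance through BPI_PlayerToAnimation, with movement gated while attacking or blocking.
; OnAttack briefly expands a sphere to damage overlapping pawns, and OnBlockChanged toggles HealthComponent damage resistance.
; Interaction messages the first overlapping BP_Interact; TryRun skips its parent call.
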(event OnStartRunning(CharacterMovement)
  (bind _animationcomponent (Variables|Default|GetAnimationComponent))
  (bind _animinstance (Variables|/Script/PaperZD.PaperZDAnimationComponent|GetAnimInstance _animationcomponent))
  (Utilities|IsValid _animinstance
    (:Is%20Valid
      (Utilities|ImplementsInterface _animinstance "/Game/SpaceGame/GameLogic/Blueprints/Interfaces/BPI_PlayerToAnimation.BPI_PlayerToAnimation_C"
        (:True
          (Class|BPIPlayertoAnimation|SetRunning(Message) _animinstance true))))))

(event OnStopRunning(CharacterMovement)
  (bind _animationcomponent (Variables|Default|GetAnimationComponent))
  (bind _animinstance (Variables|/Script/PaperZD.PaperZDAnimationComponent|GetAnimInstance _animationcomponent))
  (Utilities|IsValid _animinstance
    (:Is%20Valid
      (Utilities|ImplementsInterface _animinstance "/Game/SpaceGame/GameLogic/Blueprints/Interfaces/BPI_PlayerToAnimation.BPI_PlayerToAnimation_C"
        (:True
          (Class|BPIPlayertoAnimation|SetRunning(Message) _animinstance false))))))

(event Custom|StartCleaning
  (params (StartCleaning :type Boolean))
  (bind _animationcomponent (Variables|Default|GetAnimationComponent))
  (bind _animinstance (Variables|/Script/PaperZD.PaperZDAnimationComponent|GetAnimInstance _animationcomponent))
  (Utilities|IsValid _animinstance
    (:Is%20Valid
      (Utilities|ImplementsInterface _animinstance "/Game/SpaceGame/GameLogic/Blueprints/Interfaces/BPI_PlayerToAnimation.BPI_PlayerToAnimation_C"
        (:True
          (Class|BPIPlayertoAnimation|SetCleaning(Message) _animinstance StartCleaning))))))

(event EventBeginPlay)

(event EventTryMove
  (params (Value :type Vector%202D%20Structure))
  (bind _animationcomponent (Variables|Default|GetAnimationComponent))
  (bind _animinstance (Variables|/Script/PaperZD.PaperZDAnimationComponent|GetAnimInstance _animationcomponent))
  ;[0 0 0] Moving
  (if (Movement|CanMove)
    (|CallParentFunction Value)
    (Utilities|IsValid _animinstance
      (:Is%20Valid
        (Utilities|ImplementsInterface _animinstance "/Game/SpaceGame/GameLogic/Blueprints/Interfaces/BPI_PlayerToAnimation.BPI_PlayerToAnimation_C"
          (:True
            (Class|BPIPlayertoAnimation|UpdateMoving(Message) _animinstance Value)))))))

(event EventTryRun
  (params (Value :type Boolean))
  ;[0 0 0] Moving
)

(event EventTryInteract
  (params (Value :type Boolean))
  (bind _capsulecomponent (Variables|Default|GetCapsuleComponent))
  (bind _overlappingactors (Collision|GetOverlappingActors _capsulecomponent "/Game/SpaceGame/GameLogic/Blueprints/Interact/BP_Interact.BP_Interact_C" :!class /Script/Engine.PrimitiveComponent))
  (bind _output (Utilities|Array|Get(acopy) _overlappingactors))
  ;[0 0 0] Interaction
  (|CallParentFunction Value)
  (if Value
    (if (Utilities|Array|IsValidIndex _overlappingactors)
      (Utilities|IsValid _output
        (:Is%20Valid
          (Utilities|ImplementsInterface _output "/Game/SpaceGame/GameLogic/Blueprints/Interfaces/BPI_Interact.BPI_Interact_C"
            (:True
              (Class|BPIInteract|Interact(Message) _output))))))))

(event OnHealthChanged(HealthComponent)
  (params (NewHealth :type Float%20%28single-precision%29) (HealthDelta :type Float%20%28single-precision%29))
  (Development|PrintString (Utilities|String|ToString(Float) NewHealth)))

(event EventTryAttack
  (params (Value :type Boolean))
  (bind _animationcomponent (Variables|Default|GetAnimationComponent))
  (bind _animinstance (Variables|/Script/PaperZD.PaperZDAnimationComponent|GetAnimInstance _animationcomponent))
  ;[0 0 0] Attack
  (|CallParentFunction Value)
  (if Value
    (if (not (Variables|Attack|GetIsAttacking))
      (Variables|Attack|SetIsAttacking true)
      (Utilities|IsValid _animinstance
        (:Is%20Valid
          (Utilities|ImplementsInterface _animinstance "/Game/SpaceGame/GameLogic/Blueprints/Interfaces/BPI_PlayerToAnimation.BPI_PlayerToAnimation_C"
            (:True
              (Class|BPIPlayertoAnimation|StartAttacking(Message) _animinstance))))))))

(event EventOnAttackingFinished
  ;[0 0 0] Attack
  (Variables|Attack|SetIsAttacking false))

(event EventOnAttack
  ;[0 0 0] Attack
  (Action|Attack))

(event EventTryBlock
  (params (Value :type Boolean))
  (bind _animationcomponent (Variables|Default|GetAnimationComponent))
  (bind _animinstance (Variables|/Script/PaperZD.PaperZDAnimationComponent|GetAnimInstance _animationcomponent))
  ;[0 0 0] Block
  (|CallParentFunction Value)
  (Utilities|IsValid _animinstance
    (:Is%20Valid
      (Utilities|ImplementsInterface _animinstance "/Game/SpaceGame/GameLogic/Blueprints/Interfaces/BPI_PlayerToAnimation.BPI_PlayerToAnimation_C"
        (:True
          (Class|BPIPlayertoAnimation|ChangeBlocking(Message) _animinstance Value))))))

(event EventOnBlockingChanged
  (params (IsBlocking :type Boolean))
  ;[0 0 0] Block
  (Variables|Attack|SetIsBlocking IsBlocking))

(event EventOnBlockChanged
  (params (Active :type Boolean))
  (bind _healthcomponent (Variables|Default|GetHealthComponent))
  ;[0 0 0] Block
  (Utilities|IsValid _healthcomponent
    (:Is%20Valid
      (Class|BGCHealthComponent|SetDamageResistance _healthcomponent (Math|Float|SelectFloat 0.5 0.0 Active)))))

(fn ConstructionScript)

(fn Attack
  (Components|Sphere|SetSphereRadius (Variables|Default|GetAttackCollision) (Variables|Attack|GetBaseAttackRange) true)
  (for _array_element (Collision|GetOverlappingActors (Variables|Default|GetAttackCollision) "/Script/Engine.Pawn" :!class /Script/Engine.PrimitiveComponent)
    (if (!= _array_element self)
      (Game|Damage|ApplyDamage _array_element (Variables|Attack|GetBaseDamage) 0 self)))
  (Components|Sphere|SetSphereRadius (Variables|Default|GetAttackCollision) 0.0 true))

(fn CanMove
  (return (and (not (Variables|Attack|GetIsAttacking)) (not (Variables|Attack|GetIsBlocking)))))