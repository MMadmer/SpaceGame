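; BP_Counter_NPC is a counter level object that counts the deaths of its target NPCs.
; On BeginPlay it binds to the health component OnDeath event of each BP_NPCBase in Targets, and each death calls the inherited AddCount.
; Its Enable override runs the parent logic, destroys every valid actor in EnableTargets and ActivateTargets, and prints a debug string.
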(event Custom|OnDeath
  (CallFunction|AddCount))

(event EventBeginPlay
  (|CallParentFunction)
  (for _array_element (Variables|Default|GetTargets)
    (bind _asbp_npcbase (Utilities|Casting|CastToBP_NPCBase _array_element))
    (Utilities|IsValid (Actor|GetComponentbyClass _asbp_npcbase "/Script/BaseGameComponents.BGCHealthComponent")
      (:Is%20Valid
        (EventDispatchers|AssignOnDeath (Actor|GetComponentbyClass _asbp_npcbase "/Script/BaseGameComponents.BGCHealthComponent") (delegate Custom|OnDeath))))))

(event EventEnable
  (|CallParentFunction)
  (for _array_element (Variables|Default|GetEnableTargets)
    (Utilities|IsValid _array_element
      (:Is%20Valid
        (Actor|DestroyActor _array_element))))
  (for _array_element_2 (Variables|Default|GetActivateTargets)
    (Utilities|IsValid _array_element_2
      (:Is%20Valid
        (Actor|DestroyActor _array_element_2))))
  (Development|PrintString "Hello"))

(fn ConstructionScript
  (|CallParentFunction))