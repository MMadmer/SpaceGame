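; BP_Counter is a level logic object that triggers linked targets once its count reaches a set number.
; AddCount increments CurrentCount and calls Enable only when it exactly equals TargetCount, so further increments do not re-trigger it.
; Enable sends EnableMessage to each of the EnableTargets, then ActivateMessage to each of the ActivateTargets.
; ShowConnections flushes persistent debug lines and draws the links to both target lists in white.
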(event Custom|ShowConnections
  ;[0.07292 0.2169 1] Debug
  (Rendering|Debug|FlushPersistentDebugLines)
  (CallFunction|ShowConnect self (Variables|Default|GetEnableTargets) "(R=1.000000,G=1.000000,B=1.000000,A=1.000000)")
  (CallFunction|ShowConnect self (Variables|Default|GetActivateTargets) "(R=1.000000,G=1.000000,B=1.000000,A=1.000000)"))

(event EventBeginPlay)

(event EventEnable
  (for _array_element (Variables|Default|GetEnableTargets)
    (Class|BPILevelTools|Enable(Message) _array_element))
  (for _array_element_2 (Variables|Default|GetActivateTargets)
    (Class|BPILevelTools|Activate(Message) _array_element_2)))

(fn ConstructionScript)

(fn AddCount
  (bind _currentcount (Variables|Count|GetCurrentCount))
  (Math|Integer|IncrementInt _currentcount
    (:%20%20
      (if (== _currentcount (Variables|Count|GetTargetCount))
        (CallFunction|Enable)))))