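; BP_Spawner is a level-object Blueprint that spawns an actor of a configurable SpawnClass at its own transform.
; It spawns on BeginPlay when ActiveOnStart is set, and again whenever its Enable event is called.
; Both events route through a Spawn function, which returns the new actor or prints a message if the class is invalid.
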(event EventBeginPlay
  (if (Variables|Default|GetActiveOnStart)
    (CallFunction|Spawn)))

(event EventEnable
  (CallFunction|Spawn))

(fn ConstructionScript)

(fn Spawn
  (if (Utilities|IsValidClass (Variables|Default|GetSpawnClass))
    (bind _returnvalue (Game|SpawnActorfromClass (Variables|Default|GetSpawnClass) (Transformation|GetActorTransform) "Undefined" "MultiplyWithRoot" 0 0))
    (return _returnvalue)
    (else
      (Development|PrintString "Spawn class not valid" true true "(R=1.000000,G=0.405365,B=0.000000,A=1.000000)" 5.0))))