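; Flipbook-sprite enemy NPC that behaves either as a roaming schoolboy or as a melee chaser of the player.
; Schoolboys loop AIMoveTo between random targets and spawn BP_Mama at random intervals; others chase and damage overlapping players, pausing movement to attack.
; HealthComponent events update a widget health bar.
; On death, it switches to a walk flipbook, heads to a random exit and destroys itself on arrival.
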(event OnDeath(HealthComponent)
  (bind _exittagets (Variables|Default|GetExitTagets))
  (Variables|Default|SetCanMama false)
  (Variables|Default|SetDead? true)
  (Variables|/Script/Engine.CharacterMovementComponent|SetMaxWalkSpeed (Variables|Character|GetCharacterMovement) (Variables|Default|GetWalkSpeed))
  (Sprite|SetFlipbook (Variables|Default|GetSprite) "/Game/SpaceGame/Assets/Animations/Girl/Walk/Front/FB_GirlWalkFront.FB_GirlWalkFront")
  (Class|NavMovementComponent|StopActiveMovement (Variables|Character|GetCharacterMovement))
  (AI|AIMoveTo self "15.000000,15.000000,15.000000" (Utilities|Array|Get(acopy) _exittagets (Math|Random|RandomIntegerinRange 0 (- (Utilities|Array|Length _exittagets) 1))) 5.0 false :!label _label
    (:OnSuccess
      (Actor|DestroyActor))
    (:OnFail
      (goto _label))))

(event OnHealthChanged(HealthComponent)
  (params (NewHealth :type Float%20%28single-precision%29) (HealthDelta :type Float%20%28single-precision%29))
  (Progress|SetPercent (Variables|/Game/SpaceGame/GameLogic/Blueprints/UI/Widgets/Base/WBP_EnemyHealthBar.WBP_EnemyHealthBar_C|GetHealthBar (Variables|Default|GetWBP%20Enemy%20Health%20Bar)) (/ NewHealth (Variables|/Script/BaseGameComponents.BGCHealthComponent|GetMaxHealth (Variables|Default|GetHealth%20Component)))))

(event Custom|StartChasing
  (AI|AIMoveTo self "5.000000,5.000000,5.000000" (Variables|Default|GetAs%20BP%20SGPlayer) 5.0 false :!label _label
    (:OnSuccess
      (CallFunction|Attack)
      (CallFunction|StartChasing))
    (:OnFail
      (goto _label))))

(event Custom|RunToExit
  (bind _tagets (Variables|Default|GetTagets))
  (bind _dead_ (Variables|Default|GetDead?))
  (AI|AIMoveTo self "15.000000,15.000000,15.000000" (Utilities|Array|Get(acopy) _tagets (Math|Random|RandomIntegerinRange 0 (- (Utilities|Array|Length _tagets) 1))) 5.0 false :!label _label
    (:OnSuccess
      (if (not _dead_)
        (if (Variables|Default|GetIsSchoolBoy)
          (Utilities|FlowControl|Delay 0.5)
          (goto _label)
          (else
            (CallFunction|StartChasing :!label _label_2)))))
    (:OnFail
      (if (not _dead_)
        (if (Variables|Default|GetIsSchoolBoy)
          (goto _label)
          (else
            (goto _label_2)))))))

(event Custom|Attack
  (bind _sprite (Variables|Default|GetSprite))
  (bind _charactermovement (Variables|Character|GetCharacterMovement))
  (bind _sphere (Variables|Default|GetSphere))
  (bind _overlappingactors (Collision|GetOverlappingActors _sphere "/Game/SpaceGame/GameLogic/Blueprints/Player/BP_SGPlayer.BP_SGPlayer_C" :!class /Script/Engine.PrimitiveComponent))
  (bind _output (Utilities|Array|Get(acopy) _overlappingactors))
  (if (Variables|Default|GetCanAttack?)
    (Utilities|IsValid _output
      (:Is%20Valid
        (Game|Damage|ApplyDamage _output 25.0 0 0)
        (Variables|Default|SetCanAttack? false)
        (Variables|/Script/Engine.CharacterMovementComponent|SetMaxWalkSpeed _charactermovement 0.0)
        (Sprite|SetFlipbook _sprite "/Game/SpaceGame/Assets/Animations/Girl/Attack/FB_GirlAttack.FB_GirlAttack")
        (if (Variables|Default|GetIsGirl)
          (Transformation|AddLocalOffset _sprite (Math|Vector|MakeVector 0.0 0.0 (Variables|Default|GetAttackOffset)) false false)
          (Development|PrintString "Attack")
          (Utilities|FlowControl|Delay (Variables|Default|GetAttackSpeed))
          (Sprite|SetFlipbook (Variables|Default|GetSprite) "/Game/SpaceGame/Assets/Animations/Girl/Run/Front/PF_GirlRunFront.PF_GirlRunFront")
          (Variables|Default|SetCanAttack? true)
          (Variables|/Script/Engine.CharacterMovementComponent|SetMaxWalkSpeed _charactermovement (Variables|Default|GetRunSpeed))
          (if (Variables|Default|GetIsGirl)
            (Transformation|AddLocalOffset (Variables|Default|GetSprite) (Math|Vector|MakeVector 0.0 0.0 (* (Variables|Default|GetAttackOffset) -1.0)) false false)))))))

(event Custom|CreateMama
  (Utilities|FlowControl|Delay (Math|Random|RandomFloatinRange (Variables|Default|GetKDToMamaMin) (Variables|Default|GetKDToMamaMax)) :!label _label)
  (if (Variables|Default|GetCanMama)
    (Game|SpawnActorfromClass "/Game/SpaceGame/GameLogic/Blueprints/Interact/BP_Mama.BP_Mama_C" (Math|Transform|MakeTransform (Transformation|GetWorldLocation (Variables|Default|GetSprite)) "0, 0, 0" "1.000000,1.000000,1.000000") "Undefined" "MultiplyWithRoot" 0 0)
    (goto _label)))

(event EventTick
  (params (DeltaSeconds :type Float%20%28single-precision%29)))

(event EventBeginPlay
  (|CallParentFunction)
  (CallFunction|ChangeType)
  (bind _returnvalue (UserInterface|CreateWidget "/Game/SpaceGame/GameLogic/Blueprints/UI/Widgets/Base/WBP_EnemyHealthBar.WBP_EnemyHealthBar_C"))
  (bind _output_get (Variables|Default|SetWBP%20Enemy%20Health%20Bar _returnvalue))
  (Progress|SetPercent (Variables|/Game/SpaceGame/GameLogic/Blueprints/UI/Widgets/Base/WBP_EnemyHealthBar.WBP_EnemyHealthBar_C|GetHealthBar _output_get) (/ (Class|BGCHealthComponent|GetHealth (Variables|Default|GetHealth%20Component)) 1e+02))
  (UserInterface|SetWidget (Variables|Default|Gete) (Variables|Default|GetWBP%20Enemy%20Health%20Bar)))

(fn ConstructionScript
  (if (Variables|Default|GetIsABoy)
    (Variables|/Script/BaseGameComponents.BGCHealthComponent|SetMaxHealth (Variables|Default|GetHealth%20Component) 1e+02)))

(fn ChangeType
  (if (Variables|Default|GetIsSchoolBoy)
    (CallFunction|RuntoExit)
    (Variables|Default|SetCanMama true)
    (CallFunction|CreateMama)
    (else
      (CallFunction|StartChasing)
      (Variables|Default|SetCanMama false))))