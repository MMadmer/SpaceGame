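; BP_Door is an interactable 2D door that swings open and closed.
; Each Interact event alternates through a FlipFlop between playing and reversing the OpenDoor timeline.
; The timeline drives a lerp on the PaperSprite's relative yaw, swinging it around the vertical axis while pitch stays fixed to keep the sprite turned 90 degrees.
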(event EventBeginPlay
  (|CallParentFunction) ; This node is disabled and will not be called.\nDrag off pins to build functionality.
)

(event Collision|EventActorBeginOverlap
  (params (OtherActor :type Actor%20Object%20Reference))
  (|CallParentFunction OtherActor) ; This node is disabled and will not be called.\nDrag off pins to build functionality.
)

(event EventTick
  (params (DeltaSeconds :type Float%20%28single-precision%29))
  (|CallParentFunction DeltaSeconds) ; This node is disabled and will not be called.\nDrag off pins to build functionality.
)

(event EventInteract
  (Utilities|FlowControl|FlipFlop
    (:A
      (bind _newtrack_0 (Timeline|OpenDoor Play)
        (:Update
          (Transformation|SetRelativeRotation (Variables|Default|GetPaperSprite) (Math|Rotator|MakeRotator 0.0 9e+01 (Math|Float|Lerp 0.0 -1.2e+02 _newtrack_0)) false false))))
    (:B
      (Timeline|OpenDoor Reverse))))

(fn ConstructionScript
  (|CallParentFunction))