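; BP_Mama is a one-time interactable that the player cleans up, adding to the cleared Mama count in BP_SGPlayerState.
; Overlap with component A toggles the interact flag and prompt widget for PlayerRef.
; Interact plays the WBP_Interact animation, then briefly zeroes walk speed while the player cleans.
; It then restores speed, calls the empty Other event, updates the player state and destroys itself.
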(event OnComponentBeginOverlap(a)
  (params (OverlappedComponent :type Primitive%20Component%20Object%20Reference) (OtherActor :type Actor%20Object%20Reference) (OtherComp :type Primitive%20Component%20Object%20Reference) (OtherBodyIndex :type Integer) (bFromSweep :type Boolean) (SweepResult :type Hit%20Result%20Structure%20%28by%20ref%29))
  (if (== OtherActor (Variables|Default|GetPlayerRef))
    (Variables|Default|SetCanINteract true)
    (Rendering|SetVisibility (Variables|Default|GetWidget) true false)))

(event OnComponentEndOverlap(a)
  (params (OverlappedComponent :type Primitive%20Component%20Object%20Reference) (OtherActor :type Actor%20Object%20Reference) (OtherComp :type Primitive%20Component%20Object%20Reference) (OtherBodyIndex :type Integer))
  (if (== OtherActor (Variables|Default|GetPlayerRef))
    (Variables|Default|SetCanINteract false)
    (Rendering|SetVisibility (Variables|Default|GetWidget) false false)))

(event Custom|Other)

(event EventBeginPlay
  (|CallParentFunction))

(event EventTick
  (params (DeltaSeconds :type Float%20%28single-precision%29))
  (if (Variables|Default|GetCanINteract)
    (Development|PrintString "CanInteract" true true "(R=0.000000,G=0.660000,B=1.000000,A=1.000000)" 0.1 "6")))

(event EventInteract
  (bind _playerref (Variables|Default|GetPlayerRef))
  (bind _playerref_2 (Variables|Default|GetPlayerRef))
  (bind _charactermovement (Variables|/Script/Engine.Character|GetCharacterMovement _playerref))
  (bind _playerstate (Variables|/Script/Engine.Pawn|GetPlayerState _playerref_2))
  (Utilities|FlowControl|DoOnce false
    (:Completed
      (bind _aswbp_interact (Utilities|Casting|CastToWBP_Interact (UserInterface|GetWidget (Variables|Default|GetWidget))))
      (Default|PlayAnim _aswbp_interact true)
      (Utilities|IsValid (Variables|Default|GetPlayerRef)
        (:Is%20Valid
          (Default|StartCleaning (Variables|Default|GetPlayerRef) true)
          (Variables|Default|SetBase%20Walk%20Speed (Variables|/Script/Engine.CharacterMovementComponent|GetMaxWalkSpeed _charactermovement))
          (Variables|/Script/Engine.CharacterMovementComponent|SetMaxWalkSpeed _charactermovement 0.0)
          (Utilities|FlowControl|Delay 1.0)
          (Default|StartCleaning (Variables|Default|GetPlayerRef) false)
          (Variables|/Script/Engine.CharacterMovementComponent|SetMaxWalkSpeed (Variables|/Script/Engine.Character|GetCharacterMovement (Variables|Default|GetPlayerRef)) (Variables|Default|GetBase%20Walk%20Speed))
          (CallFunction|Other)
          (Utilities|IsValid _playerstate
            (:Is%20Valid
              (bind _asbp_sgplayer_state (Utilities|Casting|CastToBP_SGPlayerState _playerstate)
                (:then
                  (Default|AddClearedMama _asbp_sgplayer_state 1))
                (:CastFailed
                  _))
              (Actor|DestroyActor))))))))

(fn ConstructionScript
  (Rendering|SetVisibility (Variables|Default|Geta) true true))